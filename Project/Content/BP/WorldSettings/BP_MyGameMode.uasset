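; Game mode that tracks a numbered current world and shows only the BP_Tasks actors belonging to it.
; AddTask tags a task with "Level_N" from the current world index, which starts at zero and is exposed through GetCurrentWorld.
; NextLevel and PreviousLevel shift the index without bounds checks, print it, and call TasksHidenShow.
; That function compares each task's first tag, toggling visibility and mesh collision instead of loading separate maps.
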(event `self.ReceiveBeginPlay`
  ;[1 1 1] Создаём первый мир
  (set `self.CurrentWorld` 0))

(event `/Game/BP/WorldSettings/Interfases/BPI_GameMode.AddTask`
  (params (Task :type "/Game/BP/Objects/BP_Tasks Object Reference"))
  ;[1 1 1] Присваиваем тег задаче, в зависимости от номера мира
  (set `Actor.Tags` (`|MakeArray` (`KismetStringLibrary.Conv_StringToName` (`KismetTextLibrary.Conv_TextToString` (`|FormatText` "Level_{n}" (`self.CurrentWorld`))))) Task))

(event `/Game/BP/WorldSettings/Interfases/BPI_GameMode.NextLevel`
  (bind _currentworld (`self.CurrentWorld`))
  (`/Engine/EditorBlueprintResources/StandardMacros.IncrementInt` _currentworld
    (:`  `
      (`self.TasksHidenShow`)
      (`KismetSystemLibrary.PrintText` (`|FormatText` "{n} Мир" _currentworld)))))

(event `/Game/BP/WorldSettings/Interfases/BPI_GameMode.PreviousLevel`
  (bind _currentworld (`self.CurrentWorld`))
  (`/Engine/EditorBlueprintResources/StandardMacros.DecrementInt` _currentworld
    (:`  `
      (`self.TasksHidenShow`)
      (`KismetSystemLibrary.PrintText` (`|FormatText` "{n} Мир" _currentworld)))))

(fn `GetCurrentWorld`
  (returns (CurrentWorld :type Integer))
  (return (`self.CurrentWorld`)))

(fn `TasksHidenShow`
  (bind _task (`self.Task`))
  (bind _staticmesh (`/Game/BP/Objects/BP_Tasks.StaticMesh` _task))
  ;[1 1 1] Перебераем все задачи, показываем только задачи с нужным тегом, остальные скрываем
  (bind _outactors (`GameplayStatics.GetAllActorsOfClass` "/Game/BP/Objects/BP_Tasks.BP_Tasks_C"))
  (for _array_element _outactors
    (bind _output_get (set `self.Task` _array_element))
    (if (== (`|GetArrayItem` (`Actor.Tags` _output_get)) (`KismetStringLibrary.Conv_StringToName` (`KismetTextLibrary.Conv_TextToString` (`|FormatText` "Level_{n}" (`self.CurrentWorld`)))))
      (`self.SetActorHiddenInGame` _task false)
      (`PrimitiveComponent.SetCollisionEnabled` _staticmesh "QueryAndPhysics")
      (else
        (`self.SetActorHiddenInGame` _task true)
        (`PrimitiveComponent.SetCollisionEnabled` _staticmesh "NoCollision"))))
  (return))

(fn `UserConstructionScript`)