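; BP_Tasks is a task actor that holds a resource point count, shown on floating text that turns toward the player every tick.
; On BeginPlay it registers with the game mode and aims its arrow at the nearest other task sharing its first tag, caching that task.
; A bound resource-reduction event decrements the points down to zero and refreshes the text, while SetPoints clamps external writes to a fixed range.
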(event `self.ReceiveBeginPlay`
  (bind _arrow (`self.Arrow`))
  (message `/Game/BP/WorldSettings/Interfases/BPI_GameMode.AddTask` (`GameplayStatics.GetGameMode`) self)
  ;[1 1 1] Находим близжайшее задание и поворачиваем в том направлении стрелку
  (bind _taskoutput (`self.FindSourceWithMinDistantion`))
  (bind _output_get (set `self.TaskWithMinDistanse` _taskoutput))
  (`SceneComponent.K2_SetWorldRotation` _arrow (`KismetMathLibrary.FindLookAtRotation` (`SceneComponent.K2_GetComponentLocation` _arrow) (`SceneComponent.K2_GetComponentLocation` (`/Game/BP/Objects/BP_Tasks.Arrow` _output_get))) false false)
  ;[1 1 1] Слушаем делегат, при срабатывании которого ресурсы уменьшаются
  (add `self.ResourceReduction` (delegate `ReductionPoints`)))

(event `ReductionPoints`
  ;[1 1 1] Слушаем делегат, при срабатывании которого ресурсы уменьшаются
  (if (> (`self.Points`) 0)
    (set `self.Points` (- (`self.Points`) 1))
    (`TextRenderComponent.K2_SetText` (`self.Text`) (`KismetTextLibrary.Conv_ByteToText` (`self.Points`)))))

(event `self.ReceiveTick`
  (params (DeltaSeconds :type "Float (single-precision)"))
  ;[1 1 1] Поворот текста количества ресурсов к игроку
  (`SceneComponent.K2_SetWorldRotation` (`self.Text`) (`KismetMathLibrary.FindLookAtRotation` (`SceneComponent.K2_GetComponentLocation` (`self.Text`)) (`self.K2_GetActorLocation` (`GameplayStatics.GetPlayerCharacter` 0))) false false))

(fn `ClampByte`
  (params (Value :type Byte) (Max :type Byte) (Min :type Byte))
  (returns (OutValue :type Byte))
  (if (> Value Max)
    (return Max)
    (elif (< Value Min)
      (return Min)
      (else
        (return Value)))))

(fn `FindSourceWithMinDistantion`
  (returns (TaskOutput :type "/Game/BP/Objects/BP_Tasks Object Reference"))
  (locals (MinDistanceToSource :type "Float (double-precision)" :default -1.0) (Task :type "/Game/BP/Objects/BP_Tasks Object Reference"))
  (set `local.MinDistanceToSource` -1.0)
  (set `local.Task` self)
  (bind _outactors (`GameplayStatics.GetAllActorsOfClass` "BP_Tasks_C"))
  (for _array_element _outactors
    ;[1 1 1] Проверяем 3 условия: задача не является собой, тэги задач совпадают, было ли найдено растояние больше 0, растояние меньше текущего значения переменной MinDistanceToSource
    (if (!= _array_element self)
      (if (== (`|GetArrayItem` (`self.Tags`)) (`|GetArrayItem` (`Actor.Tags` _array_element)))
        (if (< (`local.MinDistanceToSource`) 0.0)
          (set `local.Task` _array_element :!label _label)
          (bind _returnvalue (`self.GetDistanceTo` _array_element))
          (set `local.MinDistanceToSource` _returnvalue)
          (elif (< _returnvalue (`local.MinDistanceToSource`))
            (goto _label))))))
  (return (`local.Task`)))

(fn `GetPoints`
  (returns (Points :type Byte))
  (return (`self.Points`)))

(fn `GetTaskWithMinDistanse`
  (returns (TaskWithMinDistanse :type "/Game/BP/Objects/BP_Tasks Object Reference"))
  (return (`self.TaskWithMinDistanse`)))

(fn `SetPoints`
  (params (InputPoint :type Byte))
  (returns (Output_Get :type Byte))
  (bind _output_get (set `self.Points` (`self.ClampByte` InputPoint 100)))
  (return _output_get))

(fn `UserConstructionScript`
  (`TextRenderComponent.K2_SetText` (`self.Text`) (`KismetTextLibrary.Conv_ByteToText` (`self.Points`))))