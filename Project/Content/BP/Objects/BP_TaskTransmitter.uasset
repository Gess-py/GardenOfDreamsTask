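; BP_TaskTransmitter is a task object that gradually draws resource points from another task.
; On BeginPlay it starts a looping one-second timer, after its construction script has zeroed its points.
; Each tick of that timer adds a point, updates its text and calls ResourceReduction on the task from GetTaskWithMinDistanse.
; The timer stops when its own points exceed 100 or that source task has none left.
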(event `self.ReceiveBeginPlay`
  (`parent.ReceiveBeginPlay`)
  ;[1 1 1] Запускаем таймер, проверяем условия чтоб количесво ресурсов не выходило за пределы (0, 100) в задании и в задании-цели, затем добавляем ресурсы к заданию и вызываем делегат ResourseReduction в задании-цели
  (bind _returnvalue (`KismetSystemLibrary.K2_SetTimerDelegate` (delegate `AddPoints`) 1.0 true))
  (set `self.TimerAddPoints` _returnvalue))

(event `AddPoints`
  ;[1 1 1] Запускаем таймер, проверяем условия чтоб количесво ресурсов не выходило за пределы (0, 100) в задании и в задании-цели, затем добавляем ресурсы к заданию и вызываем делегат ResourseReduction в задании-цели
  (if (<= (`self.GetPoints`) 100)
    (if (> (`self.GetPoints` (`self.GetTaskWithMinDistanse`)) 0)
      (bind _output_get (`self.SetPoints` (+ (`self.GetPoints`) 1)))
      (`TextRenderComponent.K2_SetText` (`self.Text`) (`KismetTextLibrary.Conv_ByteToText` _output_get))
      (`self.ResourceReduction` (`self.GetTaskWithMinDistanse`))
      (else
        (`KismetSystemLibrary.K2_ClearAndInvalidateTimerHandle` (`self.TimerAddPoints`))))
    (else
      (`KismetSystemLibrary.K2_ClearAndInvalidateTimerHandle` (`self.TimerAddPoints`)))))

(fn `UserConstructionScript`
  (`self.SetPoints` 0)
  (`parent.UserConstructionScript`))