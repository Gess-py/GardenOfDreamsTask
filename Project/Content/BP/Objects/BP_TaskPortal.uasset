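; BP_TaskPortal is a portal object that keeps one resource point count synchronized across every task portal in the level.
; It extends a parent that supplies Points, and its construction script seeds them from PointsForAllPortals.
; Each Tick compares the two values; on a mismatch, it finds all portals with GetAllActorsOfClass and copies its count to each.
; The other portals then update their own Points and text display through SetPortalPoint.
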(event `self.ReceiveBeginPlay`
  (`parent.ReceiveBeginPlay`))

(event `self.ReceiveTick`
  (params (DeltaSeconds :type "Float (single-precision)"))
  (`parent.ReceiveTick` DeltaSeconds)
  ;[1 1 1] Проверяем изменилась ли количество ресурсов в данном портале, обновляем у всех порталов значение PointsForAllPortals и вызываем событие обновления ресурсов так же у всех кроме его самого
  (if (!= (`self.PointsForAllPortals`) (`self.GetPoints`))
    (bind _outactors (`GameplayStatics.GetAllActorsOfClass` "BP_TaskPortal_C"))
    (for _array_element _outactors
      (`self.SetPointsForAllPortals` _array_element (`self.GetPoints`))
      (if (!= _array_element self)
        (`self.SetPortalPoint` _array_element)))))

(event `SetPortalPoint`
  ;[1 1 1] Обновление значения ресурсов
  (bind _output_get (`self.SetPoints` (`self.PointsForAllPortals`)))
  (`TextRenderComponent.K2_SetText` (`self.Text`) (`KismetTextLibrary.Conv_ByteToText` _output_get)))

(fn `GetPointsForAllPortals`
  (returns (PointsForAllPortals :type Byte))
  (return (`self.PointsForAllPortals`)))

(fn `SetPointsForAllPortals`
  (params (PointsForAllPortals :type Byte))
  (returns (Output_Get :type Byte))
  (bind _output_get (set `self.PointsForAllPortals` PointsForAllPortals))
  (return _output_get))

(fn `UserConstructionScript`
  (`self.SetPoints` (`self.PointsForAllPortals`))
  (`parent.UserConstructionScript`))